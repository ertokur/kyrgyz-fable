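; BP_AudioController is a background music player that loops through a list of songs on one audio component.
; On BeginPlay it picks a random starting song and index through separate Random reads, then plays after a short random delay with a fade-in.
; When a song finishes, it unbinds the finish event, advances the index with wraparound and re-enters the delayed play sequence, which binds the event again.
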(event Custom|OnAudioFinished_Event
  (EventDispatchers|UnbindallEventsfromOnAudioFinished (Variables|Default|GetSong))
  (Utilities|FlowControl|Sequence
    (:then_0
      (if (== (+ (Variables|Default|GetCurrentIndex) 1) (Utilities|Array|Length (Variables|Default|GetSongs)))
        (Variables|Default|SetCurrentIndex 0)
        (else
          (Math|Integer|IncrementInt (Variables|Default|GetCurrentIndex)))))
    (:then_1
      (Variables|Default|SetCurrentPlaying (Utilities|Array|Get(acopy) (Variables|Default|GetSongs) (Variables|Default|GetCurrentIndex))))
    (:then_2
      (Utilities|FlowControl|Delay (Math|Random|RandomFloatinRange 2.0 4.0))
      (Audio|Components|Audio|SetSound (Variables|Default|GetSong) (Variables|Default|GetCurrentPlaying))
      (Audio|Components|Audio|FadeIn (Variables|Default|GetSong) 5.0 1.0 0.0 "Linear" :!class /Script/Engine.AudioComponent)
      (Audio|Components|Audio|Play (Variables|Default|GetSong) 0.0)
      (EventDispatchers|AssignOnAudioFinished (Variables|Default|GetSong) (delegate Custom|OnAudioFinished_Event)))))

(event EventBeginPlay
  (bind _songs (Variables|Default|GetSongs))
  (bind (_outitem _outindex) (Utilities|Array|Random _songs))
  (Variables|Default|SetCurrentPlaying _outitem)
  (Variables|Default|SetCurrentIndex _outindex)
  (Utilities|FlowControl|Delay (Math|Random|RandomFloatinRange 2.0 4.0))
  (Audio|Components|Audio|SetSound (Variables|Default|GetSong) (Variables|Default|GetCurrentPlaying))
  (Audio|Components|Audio|FadeIn (Variables|Default|GetSong) 5.0 1.0 0.0 "Linear" :!class /Script/Engine.AudioComponent)
  (Audio|Components|Audio|Play (Variables|Default|GetSong) 0.0)
  (EventDispatchers|AssignOnAudioFinished (Variables|Default|GetSong) (delegate Custom|OnAudioFinished_Event)))

(fn ConstructionScript)